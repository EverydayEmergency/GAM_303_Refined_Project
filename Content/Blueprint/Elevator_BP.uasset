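; Elevator Blueprint that the player raises and lowers with the Interact input while standing in its trigger box.
; Box overlaps from ThirdPersonCharacter open and close a gate that filters the Interact press.
; An IsUp flag toggles between playing and reversing the Movement timeline, which lerps the Cube's relative location from its origin to ElevatorLocation.
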(event `self.ReceiveBeginPlay`
  (`self.EnableInput` (`GameplayStatics.GetPlayerController` 0)))

(event `InputAction|Interact` :consume false
  (params (Key :type "Key Structure"))
  (:`Pressed`
    (`/Engine/EditorBlueprintResources/StandardMacros.Gate` true :!label _label
      (:`Exit`
        (if (`self.isUp`)
          (`self.ElevatorReverse`)
          (else
            (`self.ElevatorMove`)))))))

(event `self.Box.OnComponentBeginOverlap`
  (params (OverlappedComponent :type "PrimitiveComponent Object Reference") (OtherActor :type "Actor Object Reference") (OtherComp :type "PrimitiveComponent Object Reference") (OtherBodyIndex :type Integer) (bFromSweep :type Boolean) (SweepResult :type "HitResult Structure (by ref)"))
  (cast `/Game/ThirdPersonBP/Blueprints/ThirdPersonCharacter` OtherActor)
  (goto _label :!via `Open`))

(event `self.Box.OnComponentEndOverlap`
  (params (OverlappedComponent :type "PrimitiveComponent Object Reference") (OtherActor :type "Actor Object Reference") (OtherComp :type "PrimitiveComponent Object Reference") (OtherBodyIndex :type Integer))
  (cast `/Game/ThirdPersonBP/Blueprints/ThirdPersonCharacter` OtherActor)
  (goto _label :!via `Close`))

(event `ElevatorMove`
  (set `self.isUp` true)
  (bind (_direction _alpha) (`Timeline|Movement` :!label _label_2)
    (:`Update`
      (`SceneComponent.K2_SetRelativeLocation` (`self.Cube`) (`KismetMathLibrary.VLerp` (0.0 0.0 0.0) (`self.ElevatorLocation`) _alpha) false false))))

(event `ElevatorReverse`
  (set `self.isUp` false)
  (goto _label_2 :!via `Reverse`))

(fn `UserConstructionScript`)