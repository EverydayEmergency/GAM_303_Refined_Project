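; LevelSpawner_BP procedurally builds a level of platform parts when play begins, starting with a plain floor and finishing with an EndFloor.
; Each middle part is a weighted random pick among plain, timed and moving floors, jump pads and elevators, made by repeating classes in an array according to PartWeighting.
; Each part spawns at SpawnLocation, then moves it to its own EndPoint, chaining the pieces together.
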(event `self.ReceiveBeginPlay`
  ;[1 1 1 1 30] Event Begin Play
  (`self.SpawnPlainFloor`)
  (for _ (range (+ (`self.SpawnNum`) 1))
    (`self.SpawnParts`))
  (`|SpawnActorFromClass` "/Game/Blueprint/EndFloor.EndFloor_C" (`KismetMathLibrary.Conv_VectorToTransform` (`self.SpawnLocation`)) "Undefined" "OverrideRootScale" null null))

(event `SpawnPlainFloor`
  ;[0 1 0 1 30] Spawn Plain Floor
  (bind _returnvalue (`|SpawnActorFromClass` "/Game/Blueprint/PlainFloor_BP.PlainFloor_BP_C" (`KismetMathLibrary.Conv_VectorToTransform` (`self.SpawnLocation`)) "Undefined" "OverrideRootScale" null null))
  (set `self.SpawnLocation` (`SceneComponent.K2_GetComponentLocation` (`/Game/Blueprint/PlainFloor_BP.EndPoint` _returnvalue))))

(event `SpawnJumpPad`
  ;[0 1 0 1 30] Spawn Jump Pad
  (bind _returnvalue (`|SpawnActorFromClass` "/Game/Blueprint/JumpPad/JumpPad_BP.JumpPad_BP_C" (`KismetMathLibrary.Conv_VectorToTransform` (`self.SpawnLocation`)) "Undefined" "OverrideRootScale" null null))
  (set `self.SpawnLocation` (`SceneComponent.K2_GetComponentLocation` (`/Game/Blueprint/JumpPad/JumpPad_BP.EndPoint` _returnvalue))))

(event `SpawnHorizontalElevator`
  ;[0 1 0 1 30] Spawn Horizontal Elevator
  (bind _returnvalue (`|SpawnActorFromClass` "/Game/Blueprint/Elevators/HorizontalElevator_BP.HorizontalElevator_BP_C" (`KismetMathLibrary.Conv_VectorToTransform` (`self.SpawnLocation`)) "Undefined" "OverrideRootScale" null null))
  (set `self.SpawnLocation` (`SceneComponent.K2_GetComponentLocation` (`/Game/Blueprint/Elevators/Elevator_BP.EndPoint` _returnvalue))))

(event `SpawnVerticalElevator`
  ;[0 1 0 1 30] Spawn Vertical Elevator
  (bind _returnvalue (`|SpawnActorFromClass` "/Game/Blueprint/Elevators/VerticalElevator_BP.VerticalElevator_BP_C" (`KismetMathLibrary.Conv_VectorToTransform` (`self.SpawnLocation`)) "Undefined" "OverrideRootScale" null null))
  (set `self.SpawnLocation` (`SceneComponent.K2_GetComponentLocation` (`/Game/Blueprint/Elevators/Elevator_BP.EndPoint` _returnvalue))))

(event `SpawnTimedFloor`
  ;[0 1 0 1 30] Spawn Timed Floor
  (bind _returnvalue (`|SpawnActorFromClass` "/Game/Blueprint/TimedFloor/TimedFloor_BP.TimedFloor_BP_C" (`KismetMathLibrary.Conv_VectorToTransform` (`self.SpawnLocation`)) "Undefined" "OverrideRootScale" null null))
  (set `self.SpawnLocation` (`SceneComponent.K2_GetComponentLocation` (`/Game/Blueprint/TimedFloor/TimedFloor_BP.EndPoint` _returnvalue))))

(event `SpawnMovingFloor`
  ;[0 1 0 1 30] Spawn Moving Floor
  (bind _returnvalue (`|SpawnActorFromClass` "/Game/Blueprint/MovingFloor/MovingFloor_BP.MovingFloor_BP_C" (`KismetMathLibrary.Conv_VectorToTransform` (`self.SpawnLocation`)) "Undefined" "OverrideRootScale" null null))
  (set `self.SpawnLocation` (`SceneComponent.K2_GetComponentLocation` (`/Game/Blueprint/MovingFloor/MovingFloor_BP.EndPoint` _returnvalue))))

(event `SpawnParts`
  (bind _parttospawn (`self.PartToSpawn`))
  ;[0 1 0 1 30] Spawn Parts
  (`self.ChoosePart`)
  (if (== _parttospawn "/Game/Blueprint/PlainFloor_BP.PlainFloor_BP_C")
    (`self.SpawnPlainFloor`)
    (elif (== _parttospawn "/Game/Blueprint/JumpPad/JumpPad_BP.JumpPad_BP_C")
      (`self.SpawnJumpPad`)
      (elif (== _parttospawn "/Game/Blueprint/Elevators/HorizontalElevator_BP.HorizontalElevator_BP_C")
        (`self.SpawnHorizontalElevator`)
        (elif (== _parttospawn "/Game/Blueprint/Elevators/VerticalElevator_BP.VerticalElevator_BP_C")
          (`self.SpawnVerticalElevator`)
          (elif (== _parttospawn "/Game/Blueprint/TimedFloor/TimedFloor_BP.TimedFloor_BP_C")
            (`self.SpawnTimedFloor`)
            (elif (== _parttospawn "/Game/Blueprint/MovingFloor/MovingFloor_BP.MovingFloor_BP_C")
              (`self.SpawnMovingFloor`))))))))

(event `ChoosePart`
  (bind _partweighting (`self.PartWeighting`))
  (bind _parts (`self.Parts`))
  ;[0 1 0 1 30] ChoosePart
  (`KismetArrayLibrary.Array_Clear` (`self.Parts`))
  (bind _keys (`BlueprintMapLibrary.Map_Keys` _partweighting))
  (for _array_element _keys
    (for _ (range (+ (`BlueprintMapLibrary.Map_Find` _partweighting _array_element) 1))
      (`KismetArrayLibrary.Array_Add` (`self.Parts`) _array_element)))
  (set `self.PartToSpawn` (`|GetArrayItem` _parts (`KismetMathLibrary.RandomIntegerInRange` 0 (`KismetArrayLibrary.Array_LastIndex` _parts)))))

(fn `UserConstructionScript`)