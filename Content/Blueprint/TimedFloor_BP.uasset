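; TimedFloor_BP is a floor actor that periodically vanishes and reappears.
; On BeginPlay a looping timer, set by the Timer variable, fires FloorAppear, which toggles the floor's visibility and the actor's collision together through a boolean flag.
; A separate FlashingColor event uses a timeline to lerp the material's Color parameter from black to white, but nothing in this graph calls it.
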(event `self.ReceiveBeginPlay`
  (`KismetSystemLibrary.K2_SetTimerDelegate` (delegate `FloorAppear`) (`self.Timer`) true))

(event `FloorAppear`
  (bind _returnvalue (not (`self.FloorInvisable`)))
  (`SceneComponent.SetHiddenInGame` (`self.Floor`) (`self.FloorInvisable`) false)
  (`self.SetActorEnableCollision` _returnvalue)
  (set `self.FloorInvisable` _returnvalue))

(event `FlashingColor`
  (bind (_direction _colorchangefloattrack) (`Timeline|ColorChange`)
    (:`Update`
      (`MeshComponent.SetVectorParameterValueOnMaterials` (`self.Floor`) "Color" (`KismetMathLibrary.Conv_LinearColorToVector` (`KismetMathLibrary.LinearColorLerp` (struct) (struct :`R` 1.0 :`G` 1.0 :`B` 1.0 :`A` 1.0) _colorchangefloattrack))))))

(fn `UserConstructionScript`)