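; Fail floor trigger that ends the game when the third-person character overlaps its Box.
; On BeginPlay it gathers all actors of the listed floor types and widens the Box in X from a padded base scale plus a floor's X scale, each floor overwriting the last rather than accumulating.
; It then centers itself in X between PlainFloor_BP's StartPoint and EndFloor's FinishLine, at height FloorZ.
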(event `GetFloors`
  ;[0 1 0] Get Floors
  (for _array_element (`self.FloorsTypes`)
    (bind _outactors (`GameplayStatics.GetAllActorsOfClass` _array_element))
    (`KismetArrayLibrary.Array_Append` (`self.Floors`) _outactors)))

(event `self.ReceiveBeginPlay`
  ;[1 1 1 1 30] Event Begin Play
  (`self.SetScale`)
  (`self.Set Location`))

(event `SetScale`
  ;[0 1 0 1 30] Set Scale
  (set `self.CubeScale` (+ (`SceneComponent.RelativeScale3D` (`self.Box`)) (500.0 0.0 0.0)))
  (`self.GetFloors`)
  (for _array_element (`self.Floors`)
    (bind _returnvalue_x (`KismetMathLibrary.BreakVector` (`self.GetActorRelativeScale3D` _array_element)))
    (`SceneComponent.SetRelativeScale3D` (`self.Box`) (+ (`KismetMathLibrary.MakeVector` _returnvalue_x) (`self.CubeScale`)))))

(event `Set Location`
  (bind _returnvalue_x (`KismetMathLibrary.BreakVector` (`KismetMathLibrary.VLerp` (`self.StartLocation`) (`self.EndLocation`) 0.5)))
  ;[0 1 0 1 30] Set Location
  (bind _returnvalue (`GameplayStatics.GetActorOfClass` "/Game/Blueprint/PlainFloor_BP.PlainFloor_BP_C"))
  (bind _returnvalue_x_2 (`KismetMathLibrary.BreakVector` (`SceneComponent.K2_GetComponentLocation` (`/Game/Blueprint/PlainFloor_BP.StartPoint` _returnvalue))))
  (set `self.StartLocation` (`KismetMathLibrary.MakeVector` _returnvalue_x_2))
  (bind _returnvalue_2 (`GameplayStatics.GetActorOfClass` "/Game/Blueprint/EndFloor.EndFloor_C"))
  (bind _returnvalue_x_3 (`KismetMathLibrary.BreakVector` (`SceneComponent.K2_GetComponentLocation` (`/Game/Blueprint/EndFloor.FinishLine` _returnvalue_2))))
  (set `self.EndLocation` (`KismetMathLibrary.MakeVector` _returnvalue_x_3))
  (`SceneComponent.K2_SetWorldLocation` (`self.DefaultSceneRoot`) (`KismetMathLibrary.MakeVector` _returnvalue_x 0.0 (`self.Floor Z`)) false false))

(event `self.Box.OnComponentBeginOverlap`
  (params (OverlappedComponent :type "PrimitiveComponent Object Reference") (OtherActor :type "Actor Object Reference") (OtherComp :type "PrimitiveComponent Object Reference") (OtherBodyIndex :type Integer) (bFromSweep :type Boolean) (SweepResult :type "HitResult Structure (by ref)"))
  ;[0 1 0 1 30] On Overlap Game Ends
  (bind _asbp_third_person_character (cast `/Game/ThirdPerson/Blueprints/BP_ThirdPersonCharacter` OtherActor))
  (`/Game/ThirdPerson/Blueprints/BP_ThirdPersonCharacter.GameEnds` _asbp_third_person_character))

(fn `UserConstructionScript`)