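; Jump pad actor that launches the third-person character upward when it overlaps the Trigger component.
; The launch overrides vertical velocity with the character's jump Z velocity scaled by the pad's JumpHeight multiplier.
; After each launch, TypeChange cycles JumpType through small, medium and high, swapping the mesh material and multiplier to match, so every bounce differs from the last.
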(event `self.Trigger.OnComponentBeginOverlap`
  (params (OverlappedComponent :type "PrimitiveComponent Object Reference") (OtherActor :type "Actor Object Reference") (OtherComp :type "PrimitiveComponent Object Reference") (OtherBodyIndex :type Integer) (bFromSweep :type Boolean) (SweepResult :type "HitResult Structure (by ref)"))
  ;[1 1 1] Jump pad
  (bind _asbp_third_person_character (cast `/Game/ThirdPerson/Blueprints/BP_ThirdPersonCharacter` OtherActor))
  (`Character.LaunchCharacter` _asbp_third_person_character (`KismetMathLibrary.MakeVector` 0.0 0.0 (* (`CharacterMovementComponent.JumpZVelocity` (`Character.CharacterMovement` _asbp_third_person_character)) (`self.JumpHeight`))) false true)
  (`self.TypeChange`))

(event `TypeChange`
  ;[1 1 1] Type Change
  (if (== (`self.JumpType`) 0)
    (`PrimitiveComponent.SetMaterial` (`self.Mesh`) 0 "/Game/Blueprint/JumpPad/MediumJump_MAT_Inst.MediumJump_MAT_Inst")
    (set `self.JumpHeight` 1.75)
    (set `self.JumpType` 1)
    (elif (== (`self.JumpType`) 1)
      (`PrimitiveComponent.SetMaterial` (`self.Mesh`) 0 "/Game/Blueprint/JumpPad/HighJump_MAT_Inst.HighJump_MAT_Inst")
      (set `self.JumpHeight` 2.0)
      (set `self.JumpType` 2)
      (elif (== (`self.JumpType`) 2)
        (`PrimitiveComponent.SetMaterial` (`self.Mesh`) 0 "/Game/Blueprint/JumpPad/SmallJump_MAT_Inst.SmallJump_MAT_Inst")
        (set `self.JumpHeight` 1.5)
        (set `self.JumpType` 0)
        (else
          (`KismetSystemLibrary.PrintString` "Error"))))))

(fn `UserConstructionScript`)