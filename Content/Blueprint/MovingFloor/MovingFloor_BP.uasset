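; Moving floor actor whose Floor component travels between its relative origin and the FloorLocation offset.
; The Movement timeline drives a vector lerp that sets the floor's relative location on each update, without sweep.
; BeginPlay gives the timeline a random play rate for varied speed, and FloorMove replays it from the start whenever it finishes, looping endlessly.
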(event `self.ReceiveBeginPlay`
  ;[1 1 1] Event Begin Play
  (`TimelineComponent.SetPlayRate` (`self.Movement`) (`KismetMathLibrary.RandomFloatInRange` 1.0 2.0))
  (`self.FloorMove`))

(event `FloorMove`
  ;[1 1 1] Floor Move
  (bind (_direction _alpha) (`Timeline|Movement` :!via `PlayFromStart`)
    (:`Update`
      (`SceneComponent.K2_SetRelativeLocation` (`self.Floor`) (`KismetMathLibrary.VLerp` (0.0 0.0 0.0) (`self.FloorLocation`) _alpha) false false))
    (:`Finished`
      (`self.FloorMove`))))

(fn `UserConstructionScript`)